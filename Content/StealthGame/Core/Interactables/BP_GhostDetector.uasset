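; BP_GhostDetector is a stealth-game trap that gives away an invisible player who enters its trigger box.
; On BeginPlay it caches the player, a single BP_EnemyAI found by class lookup, and the Cone's world location.
; When the player overlaps the box it prints a debug message and, if PlayerInvisible is set, plays an explosion sound at the cone and calls MoveToDetector on that enemy.
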(event `self.ReceiveBeginPlay`
  ; Start
  (`|ExecutionSequence`
    (:`then_0`
      (bind _returnvalue (`GameplayStatics.GetActorOfClass` "/Game/StealthGame/Core/Characters/PlayerCharacter/BP_ThirdPersonCharacterCustom.BP_ThirdPersonCharacterCustom_C"))
      (set `self.PlayerActor` _returnvalue))
    (:`then_1`
      (bind _returnvalue_2 (`GameplayStatics.GetActorOfClass` "/Game/StealthGame/Characters/Enemies/BP_EnemyAI.BP_EnemyAI_C"))
      (set `self.EnemyAIActor` _returnvalue_2))
    (:`then_2`
      (set `self.DetectorPosition` (`SceneComponent.K2_GetComponentLocation` (`self.Cone`))))))

(event `self.Box.OnComponentBeginOverlap`
  (params (OverlappedComponent :type "PrimitiveComponent Object Reference") (OtherActor :type "Actor Object Reference") (OtherComp :type "PrimitiveComponent Object Reference") (OtherBodyIndex :type Integer) (bFromSweep :type Boolean) (SweepResult :type "HitResult Structure (by ref)"))
  ; Make noise if the player is near and invisible
  (if (== OtherActor (`self.PlayerActor`))
    (`KismetSystemLibrary.PrintString` "Player Detected")
    (if (`/Game/StealthGame/Core/Characters/PlayerCharacter/BP_ThirdPersonCharacterCustom.bPlayerInvisible` (`self.PlayerActor`))
      (`GameplayStatics.PlaySoundAtLocation` "/Game/StealthGame/Core/StarterContent/Audio/Explosion02.Explosion02" (`self.DetectorPosition`) (struct) 1.0 1.0 0.0 null null null null)
      (`/Game/StealthGame/Characters/Enemies/BP_EnemyAI.MoveToDetector` (`self.EnemyAIActor`)))))

(fn `UserConstructionScript`)