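; BP_GhostWall is an interactable wall that the player can pass through by dashing.
; Collider overlap events track whether the cached BP_ThirdPersonCharacterCustom is in range, while Tick polls its Dashing flag.
; A dash in range switches the Wall's collision profile to ignore pawns for a short delay, then restores blocking.
; A DoOnce prevents retriggering until that cycle finishes and resets it.
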(event `self.ReceiveBeginPlay`
  (bind _returnvalue (`GameplayStatics.GetActorOfClass` "/Game/StealthGame/Core/Characters/PlayerCharacter/BP_ThirdPersonCharacterCustom.BP_ThirdPersonCharacterCustom_C"))
  (set `self.Player` _returnvalue))

(event `self.ReceiveTick`
  (params (DeltaSeconds :type "Float (single-precision)"))
  (if (`self.bInTrigger`)
    (if (`/Game/StealthGame/Core/Characters/PlayerCharacter/BP_ThirdPersonCharacterCustom.bDashing` (`self.Player`))
      (`/Engine/EditorBlueprintResources/StandardMacros.DoOnce` false :!label _label
        (:`Completed`
          (`PrimitiveComponent.SetCollisionProfileName` (`self.Wall`) "IgnoreOnlyPawn" true)
          (`KismetSystemLibrary.Delay` 2.0)
          (`PrimitiveComponent.SetCollisionProfileName` (`self.Wall`) "BlockAllDynamic" true)
          (`self.RestEvent`))))))

(event `RestEvent`
  (goto _label :!via `Reset`))

(event `self.collider.OnComponentBeginOverlap`
  (params (OverlappedComponent :type "PrimitiveComponent Object Reference") (OtherActor :type "Actor Object Reference") (OtherComp :type "PrimitiveComponent Object Reference") (OtherBodyIndex :type Integer) (bFromSweep :type Boolean) (SweepResult :type "HitResult Structure (by ref)"))
  (if (== OtherActor (`self.Player`))
    (set `self.bInTrigger` true)))

(event `self.collider.OnComponentEndOverlap`
  (params (OverlappedComponent :type "PrimitiveComponent Object Reference") (OtherActor :type "Actor Object Reference") (OtherComp :type "PrimitiveComponent Object Reference") (OtherBodyIndex :type Integer))
  (if (== OtherActor (`self.Player`))
    (set `self.bInTrigger` false)))

(fn `UserConstructionScript`)