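; BP_ParanormalActivity is an interactable that a visible player completes by standing in its box, showing progress on a camera-facing completion bar.
; Box overlap starts a looping timer that adds clamped progress; invisible players are told to uncloak.
; Leaving zeroes the increment without clearing the timer, so re-entries stack timers.
; At maximum it marks itself completed, adds to the player's completion score once and turns off its spotlight.
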(event `self.ReceiveTick`
  (params (DeltaSeconds :type "Float (single-precision)"))
  (bind _completionbarwidget (`self.CompletionBarWidget`))
  (bind _aswbp_completion_bar (cast `/Game/StealthGame/MaterialLibrary/Widgets/WBP_CompletionBar` (`WidgetComponent.GetWidget` (`self.CompletionBarWidget`))))
  (`ProgressBar.SetPercent` (`/Game/StealthGame/MaterialLibrary/Widgets/WBP_CompletionBar.CompletionBar` _aswbp_completion_bar) (/ (`self.CurrentCompleteionValue`) (`self.MaxCompletionValue`)))
  (`SceneComponent.K2_SetWorldRotation` _completionbarwidget (`KismetMathLibrary.FindLookAtRotation` (`SceneComponent.K2_GetComponentLocation` _completionbarwidget) (`SceneComponent.K2_GetComponentLocation` (`PlayerCameraManager.TransformComponent` (`GameplayStatics.GetPlayerCameraManager` 0)))) false false))

(event `self.Box.OnComponentBeginOverlap`
  (params (OverlappedComponent :type "PrimitiveComponent Object Reference") (OtherActor :type "Actor Object Reference") (OtherComp :type "PrimitiveComponent Object Reference") (OtherBodyIndex :type Integer) (bFromSweep :type Boolean) (SweepResult :type "HitResult Structure (by ref)"))
  ; Comment
  (bind _asbp_third_person_character_custom (cast `/Game/StealthGame/Core/Characters/PlayerCharacter/BP_ThirdPersonCharacterCustom` OtherActor))
  (bind _output_get (set `self.Player` _asbp_third_person_character_custom))
  (if (`/Game/StealthGame/Core/Characters/PlayerCharacter/BP_ThirdPersonCharacterCustom.bPlayerInvisible` _output_get)
    (`KismetSystemLibrary.PrintString` "Uncloak and come back")
    (elif (not (`self.bActivityCompleted`))
      (set `self.CompletionAmount` 1.0)
      (`KismetSystemLibrary.K2_SetTimerDelegate` (delegate `AddCompletion`) (`self.GainCompletionInterval`) true)
      (`KismetSystemLibrary.PrintString` (`KismetStringLibrary.Conv_DoubleToString` (stale `AddCompletion` _output_get)))
      (`KismetSystemLibrary.PrintString` (`KismetStringLibrary.Conv_BoolToString` (stale `AddCompletion` _output_get_2))))))

(event `AddCompletion`
  ; Comment
  (bind _output_get (set `self.CurrentCompleteionValue` (`KismetMathLibrary.FClamp` (+ (`self.CurrentCompleteionValue`) (`self.CompletionAmount`)) 0.0 (`self.MaxCompletionValue`))))
  (if (== _output_get (`self.MaxCompletionValue`))
    (bind _output_get_2 (set `self.bActivityCompleted` true))
    (`/Engine/EditorBlueprintResources/StandardMacros.DoOnce` false
      (:`Completed`
        (`/Game/StealthGame/Core/Characters/PlayerCharacter/BP_ThirdPersonCharacterCustom.AddToCompletionScore` (`self.Player`))
        (`LightComponent.SetIntensity` (`self.SpotLight`) 0.0)))))

(event `self.Box.OnComponentEndOverlap`
  (params (OverlappedComponent :type "PrimitiveComponent Object Reference") (OtherActor :type "Actor Object Reference") (OtherComp :type "PrimitiveComponent Object Reference") (OtherBodyIndex :type Integer))
  ; Comment
  (if (== (`self.Player`) OtherActor)
    (set `self.CompletionAmount` 0.0)))

(fn `UserConstructionScript`)