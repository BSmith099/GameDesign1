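; Security camera for a stealth game that spots the player inside a box trigger and raises an enemy AI's ViewerCount.
; BeginPlay caches the player and a single BP_EnemyAI through GetActorOfClass, so only that one enemy is affected.
; When a visible player enters the box, the spotlight turns red and ViewerCount jumps by a fixed amount, printed for debugging.
; Player invisibility is checked only on entry; leaving restores the pale yellow light.
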(event `self.ReceiveTick`
  (params (DeltaSeconds :type "Float (single-precision)")))

(event `self.ReceiveBeginPlay`
  ; Start
  (`|ExecutionSequence`
    (:`then_0`
      (bind _returnvalue (`GameplayStatics.GetActorOfClass` "/Game/StealthGame/Core/Characters/PlayerCharacter/BP_ThirdPersonCharacterCustom.BP_ThirdPersonCharacterCustom_C"))
      (set `self.PlayerActor` _returnvalue))
    (:`then_1`
      (bind _returnvalue_2 (`GameplayStatics.GetActorOfClass` "/Game/StealthGame/Characters/Enemies/BP_EnemyAI.BP_EnemyAI_C"))
      (set `self.EnemyAIActor` _returnvalue_2))))

(event `self.Box.OnComponentBeginOverlap`
  (params (OverlappedComponent :type "PrimitiveComponent Object Reference") (OtherActor :type "Actor Object Reference") (OtherComp :type "PrimitiveComponent Object Reference") (OtherBodyIndex :type Integer) (bFromSweep :type Boolean) (SweepResult :type "HitResult Structure (by ref)"))
  (bind _enemyaiactor (`self.EnemyAIActor`))
  (bind _playeractor (`self.PlayerActor`))
  (if (== OtherActor _playeractor)
    (if (not (`/Game/StealthGame/Core/Characters/PlayerCharacter/BP_ThirdPersonCharacterCustom.bPlayerInvisible` _playeractor))
      (`LightComponent.SetLightColor` (`self.SpotLight`) (struct :`R` 1.0 :`A` 1.0) true)
      (bind _output_get (set `/Game/StealthGame/Characters/Enemies/BP_EnemyAI.ViewerCount` (+ (`/Game/StealthGame/Characters/Enemies/BP_EnemyAI.ViewerCount` _enemyaiactor) 50) _enemyaiactor))
      (`KismetSystemLibrary.PrintString` (`KismetStringLibrary.Conv_IntToString` _output_get)))))

(event `self.Box.OnComponentEndOverlap`
  (params (OverlappedComponent :type "PrimitiveComponent Object Reference") (OtherActor :type "Actor Object Reference") (OtherComp :type "PrimitiveComponent Object Reference") (OtherBodyIndex :type Integer))
  (if (== OtherActor (`self.PlayerActor`))
    (`LightComponent.SetLightColor` (`self.SpotLight`) (struct :`R` 0.989398 :`G` 1.0 :`B` 0.721553 :`A` 1.0) true)))

(fn `UserConstructionScript`)