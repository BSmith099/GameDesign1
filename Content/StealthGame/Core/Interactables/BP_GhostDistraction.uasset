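; Ghost distraction interactable for a stealth game that draws the enemy AI toward it when a visible player comes near.
; On BeginPlay it caches the player, a single BP_EnemyAI found by class lookup, and its cylinder's world location as DistractionPosition.
; When the player overlaps the sphere collider while not invisible, it registers itself as the enemy's GhostDistraction and calls MoveToDistraction.
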(event `self.ReceiveBeginPlay`
  (`|ExecutionSequence`
    (:`then_0`
      (bind _returnvalue (`GameplayStatics.GetActorOfClass` "/Game/StealthGame/Core/Characters/PlayerCharacter/BP_ThirdPersonCharacterCustom.BP_ThirdPersonCharacterCustom_C"))
      (set `self.PlayerCharacter` _returnvalue))
    (:`then_1`
      (bind _returnvalue_2 (`GameplayStatics.GetActorOfClass` "/Game/StealthGame/Characters/Enemies/BP_EnemyAI.BP_EnemyAI_C"))
      (set `self.Enemy` _returnvalue_2))
    (:`then_2`
      (set `self.DistractionPosition` (`SceneComponent.K2_GetComponentLocation` (`self.Cylinder`))))))

(event `self.SphereCollider.OnComponentBeginOverlap`
  (params (OverlappedComponent :type "PrimitiveComponent Object Reference") (OtherActor :type "Actor Object Reference") (OtherComp :type "PrimitiveComponent Object Reference") (OtherBodyIndex :type Integer) (bFromSweep :type Boolean) (SweepResult :type "HitResult Structure (by ref)"))
  (if (== OtherActor (`self.PlayerCharacter`))
    (if (not (`/Game/StealthGame/Core/Characters/PlayerCharacter/BP_ThirdPersonCharacterCustom.bPlayerInvisible` (`self.PlayerCharacter`)))
      (set `/Game/StealthGame/Characters/Enemies/BP_EnemyAI.GhostDistraction` self (`self.Enemy`))
      (`/Game/StealthGame/Characters/Enemies/BP_EnemyAI.MoveToDistraction` (`self.Enemy`)))))

(fn `UserConstructionScript`)